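; Rifleman character Blueprint with skills that feeds its health and skill cooldowns to a status gauge widget.
; UpdateLifeGauge casts the StatusUI widget to HPSPULTGuage and passes it current and max health from Status.
; UpdateCooldown reads the SP and ULT skill cooldowns in sequence, pushing both rates to the widget after each read.
; BeginPlay only calls the parent, and Tick, overlap and construction logic are empty.
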(event EventBeginPlay
  (|CallParentFunction))

(event Collision|EventActorBeginOverlap
  (params (OtherActor :type Actor%20Object%20Reference)))

(event EventTick
  (params (DeltaSeconds :type Float%20%28single-precision%29)))

(event EventUpdateCooldown
  (bind _ashpspultguage (Utilities|Casting|CastToHPSPULTGuage (UserInterface|GetUserWidgetObject (Variables|Default|GetStatusUI))))
  (Utilities|FlowControl|Sequence
    (:then_0
      (bind _returnvalue (Class|CCSCharacter|GetSPSkillCooldown)))
    (:then_1
      (bind _returnvalue_2 (Class|CCSCharacter|GetULTSkillCooldown))))
  (Default|UpdateCoolDown _ashpspultguage _returnvalue _returnvalue_2))

(event EventUpdateLifeGauge
  (bind _status (Variables|Default|GetStatus))
  (bind _ashpspultguage (Utilities|Casting|CastToHPSPULTGuage (UserInterface|GetUserWidgetObject (Variables|Default|GetStatusUI))))
  (Default|UpdateHP _ashpspultguage (Variables|/Script/CSProject.C_StatusComponent|GetCurHealth _status) (Variables|/Script/CSProject.C_StatusComponent|GetMaxHealth _status)))

(fn ConstructionScript)